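; Exploding barrel obstacle that detonates when hit by a first-person projectile or when Activate is called.
; Detonation plays sound and particles, deals radial damage within its Sphere's radius, then destroys the barrel.
; It chain-reacts by activating overlapping barrels, using an IsExploding flag to skip those already triggered.
; A sphere trace finds physics-simulating meshes, pushes them with a radial impulse and applies further radial damage for each.
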(event OnComponentHit(StaticMeshComponent)
  (params (HitComponent :type Primitive%20Component%20Object%20Reference) (OtherActor :type Actor%20Object%20Reference) (OtherComp :type Primitive%20Component%20Object%20Reference) (NormalImpulse :type Vector :default "0, 0, 0") (Hit :type Hit%20Result%20Structure%20%28by%20ref%29))
  (bind _sphere (Variables|Default|GetSphere))
  (bind _staticmeshcomponent (Variables|Debug|GetStaticMeshComponent))
  (bind _sphere_2 (Variables|Default|GetSphere))
  (bind _returnvalue (Transformation|GetWorldLocation _sphere_2))
  (bind _returnvalue_2 (Transformation|GetWorldLocation _sphere))
  (bind _returnvalue_3 (Components|Sphere|GetScaledSphereRadius _sphere_2))
  (bind _returnvalue_4 (Transformation|GetWorldTransform _staticmeshcomponent))
  (if (== (Utilities|GetClass OtherActor) "/Game/FirstPersonBP/Blueprints/FirstPersonProjectile.FirstPersonProjectile_C")
    (Actor|DestroyActor OtherActor)
    (Variables|Default|SetbIsExploding true)
    (Audio|PlaySoundatLocation "/Game/StarterContent/Audio/Explosion_Cue.Explosion_Cue" (Transformation|GetWorldLocation (Variables|Debug|GetStaticMeshComponent)) "0, 0, 0" 1.0 0.9 0.0 0 0 0)
    (Effects|SpawnEmitteratLocation "/Game/StarterContent/Particles/P_Explosion.P_Explosion" (.location _returnvalue_4) "0, 0, 0" "4.000000,4.000000,4.000000")
    (Utilities|FlowControl|Sequence
      (:then_0
        (Game|Damage|ApplyRadialDamage 1e+03 (.location _returnvalue_4) (Components|Sphere|GetScaledSphereRadius (Variables|Default|GetSphere)) 0 0 0 0 false "ECC_Visibility"))
      (:then_1
        ;[1 1 1] Make other barrels around this one explode
        (for _array_element (Collision|GetOverlappingActors (Variables|Default|GetSphere) "Exploding_Barrel_C" :!class /Script/Engine.PrimitiveComponent)
          (if (!= _array_element self)
            (bind _asexploding_barrel (Utilities|Casting|CastToExploding_Barrel _array_element))
            (if (not (Variables|Exploding_Barrel_C|GetbIsExploding _asexploding_barrel))
              (Variables|Exploding_Barrel_C|SetbIsExploding _asexploding_barrel true)
              (CallFunction|Activate _asexploding_barrel) ; make them explode
            ))))
      (:then_2
        ;[1 1 1] Pushback Objects
        (bind _outhits (Collision|MultiSphereTraceByChannel _returnvalue_2 _returnvalue_2 (Components|Sphere|GetScaledSphereRadius _sphere) "TraceTypeQuery1" false 0 "None" true "(R=1.000000,G=0.000000,B=0.000000,A=1.000000)" "(R=0.000000,G=1.000000,B=0.000000,A=1.000000)" 1.0))
        (for _array_element_2 _outhits
          (if (Physics|IsSimulatingPhysics (Variables|/Script/Engine.Actor|GetRootComponent (.HitActor (Collision|BreakHitResult _array_element_2))) "None")
            (bind _asstatic_mesh_component (Utilities|Casting|CastToStaticMeshComponent (Variables|/Script/Engine.Actor|GetRootComponent (.HitActor (Collision|BreakHitResult _array_element_2)))))
            (Physics|AddRadialImpulse _asstatic_mesh_component _returnvalue _returnvalue_3 (* (Variables|Default|GetExplosionStrength) (Physics|GetMass (Variables|Debug|GetStaticMeshComponent))) "RIF_Linear" true)
            (Game|Damage|ApplyRadialDamage 1e+04 _returnvalue _returnvalue_3 0 0 self 0 false "ECC_Visibility"))))
      (:then_3
        (Actor|DestroyActor)))))

(event Custom|Activate
  (bind _sphere (Variables|Default|GetSphere))
  (bind _staticmeshcomponent (Variables|Debug|GetStaticMeshComponent))
  (bind _sphere_2 (Variables|Default|GetSphere))
  (bind _returnvalue (Transformation|GetWorldLocation _sphere_2))
  (bind _returnvalue_2 (Transformation|GetWorldLocation _sphere))
  (bind _returnvalue_3 (Components|Sphere|GetScaledSphereRadius _sphere_2))
  (bind _returnvalue_4 (Transformation|GetWorldTransform _staticmeshcomponent))
  (Variables|Default|SetbIsExploding true)
  (Audio|PlaySoundatLocation "/Game/StarterContent/Audio/Explosion_Cue.Explosion_Cue" (Transformation|GetWorldLocation (Variables|Debug|GetStaticMeshComponent)) "0, 0, 0" 1.0 0.9 0.0 0 0 0)
  (Effects|SpawnEmitteratLocation "/Game/StarterContent/Particles/P_Explosion.P_Explosion" (.location _returnvalue_4) "0, 0, 0" "4.000000,4.000000,4.000000")
  (Utilities|FlowControl|Sequence
    (:then_0
      (Game|Damage|ApplyRadialDamage 1e+03 (.location _returnvalue_4) (Components|Sphere|GetScaledSphereRadius (Variables|Default|GetSphere)) 0 0 0 0 false "ECC_Visibility"))
    (:then_1
      ;[1 1 1] Make other barrels around this one explode
      (for _array_element (Collision|GetOverlappingActors (Variables|Default|GetSphere) "Exploding_Barrel_C" :!class /Script/Engine.PrimitiveComponent)
        (if (!= _array_element self)
          (bind _asexploding_barrel (Utilities|Casting|CastToExploding_Barrel _array_element))
          (if (not (Variables|Exploding_Barrel_C|GetbIsExploding _asexploding_barrel))
            (Variables|Exploding_Barrel_C|SetbIsExploding _asexploding_barrel true)
            (CallFunction|Activate _asexploding_barrel) ; make them explode
          ))))
    (:then_2
      ;[1 1 1] Pushback Objects
      (bind _outhits (Collision|MultiSphereTraceByChannel _returnvalue_2 _returnvalue_2 (Components|Sphere|GetScaledSphereRadius _sphere) "TraceTypeQuery1" false 0 "None" true "(R=1.000000,G=0.000000,B=0.000000,A=1.000000)" "(R=0.000000,G=1.000000,B=0.000000,A=1.000000)" 1.0))
      (for _array_element_2 _outhits
        (if (Physics|IsSimulatingPhysics (Variables|/Script/Engine.Actor|GetRootComponent (.HitActor (Collision|BreakHitResult _array_element_2))) "None")
          (bind _asstatic_mesh_component (Utilities|Casting|CastToStaticMeshComponent (Variables|/Script/Engine.Actor|GetRootComponent (.HitActor (Collision|BreakHitResult _array_element_2)))))
          (Physics|AddRadialImpulse _asstatic_mesh_component _returnvalue _returnvalue_3 (* (Variables|Default|GetExplosionStrength) (Physics|GetMass (Variables|Debug|GetStaticMeshComponent))) "RIF_Linear" true)
          (Game|Damage|ApplyRadialDamage 1e+04 _returnvalue _returnvalue_3 0 0 self 0 false "ECC_Visibility"))))
    (:then_3
      (Actor|DestroyActor))))

(event EventBeginPlay)

(event Collision|EventActorBeginOverlap
  (params (OtherActor :type Actor%20Object%20Reference)))

(event EventTick
  (params (DeltaSeconds :type Float%20%28single-precision%29)))

(fn ConstructionScript)