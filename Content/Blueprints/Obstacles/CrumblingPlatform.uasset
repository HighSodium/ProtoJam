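; Crumbling platform obstacle that shakes and then falls when its trigger component is overlapped while it is active.
; The overlap plays a random collapse sound and destroys the trigger so it fires only once.
; A delayed loop with a FlipFlop rumbles the mesh up and down for a set number of shakes.
; The mesh then switches to physics simulation, and the actor destroys itself after a delay.
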(event OnComponentBeginOverlap(wre)
  (params (OverlappedComponent :type Primitive%20Component%20Object%20Reference) (OtherActor :type Actor%20Object%20Reference) (OtherComp :type Primitive%20Component%20Object%20Reference) (OtherBodyIndex :type Integer) (bFromSweep :type Boolean) (SweepResult :type Hit%20Result%20Structure%20%28by%20ref%29))
  (bind _rumbledistance (Variables|Default|GetRumbleDistance))
  ;[1 1 1] Detect and fall
  (if (Variables|Default|GetbIsActive)
    (Audio|PlaySoundatLocation (.OutItem (Utilities|Array|Random (Variables|Default|GetCollapseSounds))) "0, 0, 0" "0, 0, 0" (Variables|Default|GetSoundVolume) (Variables|Default|GetSoundPitch) 0.0 0 0 0)
    (Components|DestroyComponent (Variables|Default|Getwre))
    (if (< (Variables|Default|GetShakenCount) (Variables|Default|GetShakeAmount)) :!label _label
      ;[1 1 1] Rumble
      (bind _isa (Utilities|FlowControl|FlipFlop)
        (:A
          _)
        (:B
          _))
      (Transformation|AddRelativeLocation (Variables|Debug|GetStaticMeshComponent) (Math|Vector|MakeVector 0.0 0.0 (Math|Float|SelectFloat _rumbledistance (* _rumbledistance -1.0) _isa)) false false)
      (Utilities|FlowControl|Delay (Variables|Default|GetShakeSpeed))
      (Math|Integer|IncrementInt (Variables|Default|GetShakenCount)
        (:%20%20
          (goto _label)))
      (else
        (Physics|SetSimulatePhysics (Variables|Debug|GetStaticMeshComponent) true)
        (Utilities|FlowControl|Delay (Variables|Default|GetRemoveDelay))
        (Actor|DestroyActor)))))

(event EventBeginPlay)

(event Collision|EventActorBeginOverlap
  (params (OtherActor :type Actor%20Object%20Reference)))

(event EventTick
  (params (DeltaSeconds :type Float%20%28single-precision%29)))

(fn ConstructionScript)